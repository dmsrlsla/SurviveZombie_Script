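; BP_SZPlayerController is a player controller that assigns widget interaction indices to the BP_SZMotionHandController actors in the level.
; On BeginPlay it waits briefly, then gathers every hand controller and sets each WidgetInteraction's virtual user and pointer index from its array position, giving each its own pointer.
; The authority and remote branches run identical logic, each on its locally found actors.
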(event `self.ReceiveBeginPlay`
  (`KismetSystemLibrary.Delay` 1.5)
  (`/Engine/EditorBlueprintResources/ActorMacros.Switch Has Authority`
    (:`Authority`
      (bind _outactors (`GameplayStatics.GetAllActorsOfClass` "/Game/WorkSpace/SUNGWEHYUN/BP_SZMotionHandController.BP_SZMotionHandController_C"))
      (for (_array_element _array_index) _outactors
        (bind _widgetinteraction (`/Game/WorkSpace/SUNGWEHYUN/BP_SZMotionHandController.WidgetInteraction` _array_element))
        (bind _output_get (set `WidgetInteractionComponent.VirtualUserIndex` _array_index _widgetinteraction))
        (set `WidgetInteractionComponent.PointerIndex` (`KismetMathLibrary.Conv_IntToDouble` _output_get) _widgetinteraction)))
    (:`Remote`
      (bind _outactors_2 (`GameplayStatics.GetAllActorsOfClass` "/Game/WorkSpace/SUNGWEHYUN/BP_SZMotionHandController.BP_SZMotionHandController_C"))
      (for (_array_element_2 _array_index_2) _outactors_2
        (bind _widgetinteraction_2 (`/Game/WorkSpace/SUNGWEHYUN/BP_SZMotionHandController.WidgetInteraction` _array_element_2))
        (bind _output_get_2 (set `WidgetInteractionComponent.VirtualUserIndex` _array_index_2 _widgetinteraction_2))
        (set `WidgetInteractionComponent.PointerIndex` (`KismetMathLibrary.Conv_IntToDouble` _output_get_2) _widgetinteraction_2)))))

(fn `UserConstructionScript`)