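; Game mode Blueprint for SZ that gives motion hand controllers distinct IDs and widget pointers when a player logs in.
; After a short delay on PostLogin, it loops over every BP_SZMotionHandController, using the array index as its ID and its WidgetInteraction virtual user and pointer index.
; Disconnected leftover chains hold state debug prints and waiting-for-players cleanup and start logic, none of which runs.
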(event `self.ReceiveBeginPlay`)

(event `self.K2_PostLogin`
  (params (NewPlayer :type "PlayerController Object Reference"))
  (`KismetSystemLibrary.Delay` 1.5)
  (bind _outactors (`GameplayStatics.GetAllActorsOfClass` "/Game/WorkSpace/SUNGWEHYUN/BP_SZMotionHandController.BP_SZMotionHandController_C"))
  (for (_array_element _array_index) _outactors
    (bind _widgetinteraction (`/Game/WorkSpace/SUNGWEHYUN/BP_SZMotionHandController.WidgetInteraction` _array_element))
    (bind _output_get (set `WidgetInteractionComponent.VirtualUserIndex` _array_index _widgetinteraction))
    (set `WidgetInteractionComponent.PointerIndex` (`KismetMathLibrary.Conv_IntToDouble` _output_get) _widgetinteraction)
    (`/Game/WorkSpace/SUNGWEHYUN/BP_SZMotionHandController.Set_Id` _array_element _array_index)))

(event `self.ReceiveTick`
  (params (DeltaSeconds :type "Float (single-precision)")))

(fn `UserConstructionScript`)