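; AKU ammo pickup that gives an overlapping SZCharacter one count of AKU ammo, then respawns in place.
; On pickup it clears the Ammo skeletal mesh and sets CheckAmmo, which blocks further pickups while the actor itself remains.
; Tick accumulates RespawnTime while CheckAmmo is set, then restores SettingMesh and clears the flag once CheckTime is reached.
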(event `self.ReceiveBeginPlay`
  (`SkinnedMeshComponent.SetSkinnedAssetAndUpdate` (`self.Ammo`) (`self.SettingMesh`) true))

(event `self.ReceiveActorBeginOverlap`
  (params (OtherActor :type "Actor Object Reference"))
  (bind _asszcharacter (cast `SZCharacter` OtherActor))
  (if (not (`self.checkAmmo`))
    (`SkinnedMeshComponent.SetSkinnedAssetAndUpdate` (`self.Ammo`) null true)
    (set `self.checkAmmo` true)
    (`SZCharacter.SetAmmoPlus` _asszcharacter "AKU" 1)))

(event `self.ReceiveTick`
  (params (DeltaSeconds :type "Float (single-precision)"))
  (if (`self.checkAmmo`)
    (bind _output_get (set `self.RespawnTime` (+ DeltaSeconds (`self.RespawnTime`))))
    (if (>= _output_get (`self.CheckTime`))
      (set `self.RespawnTime` 0.0)
      (`SkinnedMeshComponent.SetSkinnedAssetAndUpdate` (`self.Ammo`) (`self.SettingMesh`) true)
      (set `self.checkAmmo` false))))

(fn `UserConstructionScript`)